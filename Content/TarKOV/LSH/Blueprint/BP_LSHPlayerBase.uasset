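; BP_LSHPlayerBase is a player character Blueprint with a toggleable inventory and camera-based interaction.
; BeginPlay creates an inventory widget bound to its inventory component; the inventory input toggles it along with cursor and input mode.
; Interaction sphere-traces forward from the follow camera, either triggering a hit item's pickup event or passing another player's inventory component to the widget to open.
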(event `self.ReceiveBeginPlay`
  (bind _returnvalue (`|CreateWidget` "/Game/TarKOV/LSH/Inventory/WB_InventoryWidget.WB_InventoryWidget_C" (`self.GetPlayerController`) (`self.AC_InventoryComponent`) 50.0))
  (set `self.InventoryWidget` _returnvalue))

(event `EnhancedInput|/Game/TarKOV/LSH/Input/IA_Inventory`
  (params (ActionValue :type Boolean) (ElapsedSeconds :type "Float (double-precision)") (TriggeredSeconds :type "Float (double-precision)") (InputAction :type "InputAction Object Reference" :default "/Game/TarKOV/LSH/Input/IA_Inventory.IA_Inventory"))
  (:`Started`
    (if (`Widget.IsInViewport` (`self.InventoryWidget`))
      ;[1 1 1] 인벤UI 끄기
      (`Widget.RemoveFromParent` (`self.InventoryWidget`))
      (`WidgetBlueprintLibrary.SetInputMode_GameOnly` (`self.GetPlayerController`))
      (set `PlayerController.bShowMouseCursor` false (`self.GetPlayerController`))
      (else
        ;[1 1 1] 인벤UI 켜기
        (`UserWidget.AddToViewport` (`self.InventoryWidget`) 0)
        (`WidgetBlueprintLibrary.SetInputMode_GameAndUIEx` (`self.GetPlayerController`) (`self.InventoryWidget`) "DoNotLock" false)
        (set `PlayerController.bShowMouseCursor` true (`self.GetPlayerController`))))))

(event `EnhancedInput|/Game/TarKOV/LSH/Input/IA_Interaction`
  (params (ActionValue :type Boolean) (ElapsedSeconds :type "Float (double-precision)") (TriggeredSeconds :type "Float (double-precision)") (InputAction :type "InputAction Object Reference" :default "/Game/TarKOV/LSH/Input/IA_Interaction.IA_Interaction"))
  (bind _followcamera (`self.FollowCamera`))
  (bind _returnvalue (`SceneComponent.K2_GetComponentLocation` _followcamera))
  (:`Started`
    (bind _outhit (`KismetSystemLibrary.SphereTraceSingle` :`Start` _returnvalue :`End` (+ (* (`SceneComponent.GetForwardVector` _followcamera) 300) _returnvalue) :`Radius` 40.0 :`TraceChannel` "TraceTypeQuery2" :`DrawDebugType` "ForDuration"))
    (bind (_bblockinghit _binitialoverlap _time _distance _location _impactpoint _normal _impactnormal _physmat _hitactor) (`GameplayStatics.BreakHitResult` _outhit))
    ;[1 1 1] 아이템 인벤에 추가하기
    (bind _asbp_item (cast `/Game/TarKOV/LSH/Items/BP_Item` _hitactor)
      (:`then`
        (`/Game/TarKOV/LSH/Items/BP_Item.EatItemEvent` _asbp_item self))
      (:`CastFailed`
        ;[1 1 1] 다른사람 인벤 열기
        (bind _asbp_lshplayer_base (cast `/Game/TarKOV/LSH/Blueprint/BP_LSHPlayerBase` _hitactor))
        (`/Game/TarKOV/LSH/Inventory/WB_InventoryWidget.openOtherInven` (`self.InventoryWidget`) (`/Game/TarKOV/LSH/Blueprint/BP_LSHPlayerBase.AC_InventoryComponent` _asbp_lshplayer_base))))))

(fn `GetPlayerController`
  (returns (`AsPlayer Controller` :type "PlayerController Object Reference"))
  (return (cast `PlayerController` (`self.GetController` self) :!pure true)))

(fn `UserConstructionScript`)