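; Test player Blueprint for the inventory system, with a demo for viewing another player's inventory.
; Its event entry points are empty, and the remaining graph logic is disconnected, so it never runs.
; Those leftover chains create and toggle an inventory widget with input mode and cursor, sphere-trace from the camera, and open a hit player's inventory component.
; A helper function returns the controller cast to PlayerController.
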(event `self.ReceiveBeginPlay`)

(event `EnhancedInput|/Game/TarKOV/LSH/Input/IA_Inventory`
  (params (ActionValue :type Boolean) (ElapsedSeconds :type "Float (double-precision)") (TriggeredSeconds :type "Float (double-precision)") (InputAction :type "InputAction Object Reference" :default "/Game/TarKOV/LSH/Input/IA_Inventory.IA_Inventory")))

(event `self.CapsuleComponent.OnComponentHit`
  (params (HitComponent :type "PrimitiveComponent Object Reference") (OtherActor :type "Actor Object Reference") (OtherComp :type "PrimitiveComponent Object Reference") (NormalImpulse :type "Vector Structure") (Hit :type "HitResult Structure (by ref)"))
  ;[1 1 1] 다른사람인벤보기 (시연용)
)

(event `Key|F`
  (params (Key :type "Key Structure")))

(fn `GetPlayerController`
  (returns (`AsPlayer Controller` :type "PlayerController Object Reference"))
  (return (cast `PlayerController` (`self.GetController` self) :!pure true)))

(fn `UserConstructionScript`)